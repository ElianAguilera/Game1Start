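; BP_Door2 is a swinging door that opens automatically when the player character (BP_ThirdPersonCharacterCustom) enters its Sphere trigger and closes when that character leaves.
; Entering plays an opening sound and runs the OpenDoor timeline, whose track rotates the Door component's relative yaw in the negative direction.
; Leaving plays a closing sound and reverses the timeline from its end, so a partly opened door snaps to the end pose before closing.
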(event `self.Sphere.OnComponentBeginOverlap`
  (params (OverlappedComponent :type "PrimitiveComponent Object Reference") (OtherActor :type "Actor Object Reference") (OtherComp :type "PrimitiveComponent Object Reference") (OtherBodyIndex :type Integer) (bFromSweep :type Boolean) (SweepResult :type "HitResult Structure (by ref)"))
  (cast `/Game/Blueprints/BP_ThirdPersonCharacterCustom` OtherActor)
  (`GameplayStatics.PlaySoundAtLocation` "/Game/Audio/DoorOpening.DoorOpening" (`SceneComponent.K2_GetComponentLocation` (`self.Sphere`)) (struct) 1.0 1.0 0.0 null null null null)
  (bind (_direction _newtrack_0) (`Timeline|Open Door` :!label _label)
    (:`Update`
      (`SceneComponent.K2_SetRelativeRotation` (`self.Door`) (`KismetMathLibrary.MakeRotator` 0.0 0.0 (* _newtrack_0 -90.0)) false false))))

(event `self.Sphere.OnComponentEndOverlap`
  (params (OverlappedComponent :type "PrimitiveComponent Object Reference") (OtherActor :type "Actor Object Reference") (OtherComp :type "PrimitiveComponent Object Reference") (OtherBodyIndex :type Integer))
  (cast `/Game/Blueprints/BP_ThirdPersonCharacterCustom` OtherActor)
  (`GameplayStatics.PlaySoundAtLocation` "/Game/Audio/DoorClosing.DoorClosing" (`SceneComponent.K2_GetComponentLocation` (`self.Sphere`)) (struct) 1.0 1.0 0.0 null null null null)
  (goto _label :!via `ReverseFromEnd`))

(fn `UserConstructionScript`)