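; Patrol AI pawn that loops endlessly through actors tagged "PatrolPoint-VFXLevel" while its moves succeed.
; BeginPlay gathers the points, then GoToControlPoint moves to the current one, increments the wrapping index and re-calls itself after a short delay.
; A failed move only prints a debug string, ending the loop.
; A similar self-repeating MoveTo event follows the player character, but nothing in this file starts it.
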(event `self.ReceiveBeginPlay`
  (bind _outactors (`GameplayStatics.GetAllActorsOfClassWithTag` "/Script/Engine.Actor" "PatrolPoint-VFXLevel"))
  (`KismetSystemLibrary.PrintString` (`KismetStringLibrary.Concat_StrStr` " There are " (`KismetStringLibrary.Conv_IntToString` (`KismetArrayLibrary.Array_Length` _outactors)) " Patrol Points.") true true (struct :`G` 0.66 :`B` 1.0 :`A` 1.0) 10.0)
  (`self.GoToControlPoint`))

(event `Move To`
  (`|AIMoveTo` self (0.0 0.0 0.0) (`GameplayStatics.GetPlayerCharacter` 0) 50.0
    (:`OnSuccess`
      (`KismetSystemLibrary.PrintString` "Player! :)")
      (`KismetSystemLibrary.Delay` 1.0)
      (`self.Move To`))
    (:`OnFail`
      (`KismetSystemLibrary.PrintString` "NoPlayer"))))

(event `GoToControlPoint`
  (`|AIMoveTo` self (`self.K2_GetActorLocation` (`|GetArrayItem` (stale `self.ReceiveBeginPlay` _outactors) (`self.Current Patrol Point`))) null 50.0
    (:`OnSuccess`
      (`KismetSystemLibrary.PrintString` "Player! :)")
      (bind _result (`/Engine/EditorBlueprintResources/StandardMacros.IncrementInt` (`self.Current Patrol Point`))
        (:`  `
          (if (>= _result (`KismetArrayLibrary.Array_Length` (stale `self.ReceiveBeginPlay` _outactors)))
            (set `self.Current Patrol Point` 0))
          (`KismetSystemLibrary.Delay` 1.0)
          (`self.GoToControlPoint`))))
    (:`OnFail`
      (`KismetSystemLibrary.PrintString` "NoPlayer"))))

(fn `UserConstructionScript`)