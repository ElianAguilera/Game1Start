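; A bunker door that opens automatically when the custom third-person character enters its sphere trigger and closes when the character leaves.
; Overlap begin plays an opening sound and runs a timeline that both slides the door along X and rotates it in yaw, using separate tracks.
; Overlap end plays a closing sound and reverses that timeline from its end, even if the door is only partly open.
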(event `self.Sphere.OnComponentBeginOverlap`
  (params (OverlappedComponent :type "PrimitiveComponent Object Reference") (OtherActor :type "Actor Object Reference") (OtherComp :type "PrimitiveComponent Object Reference") (OtherBodyIndex :type Integer) (bFromSweep :type Boolean) (SweepResult :type "HitResult Structure (by ref)"))
  (cast `/Game/Blueprints/BP_ThirdPersonCharacterCustom` OtherActor)
  (`GameplayStatics.PlaySoundAtLocation` "/Game/Audio/DoorOpening.DoorOpening" (`SceneComponent.K2_GetComponentLocation` (`self.Sphere`)) (struct) 1.0 1.0 0.0 null null null null)
  (bind (_direction _newtrack_0 _newtrack_1) (`Timeline|Timeline` :!label _label)
    (:`Update`
      (`SceneComponent.K2_SetRelativeLocationAndRotation` (`self.Door`) (`KismetMathLibrary.MakeVector` (* _newtrack_1 -360.0)) (`KismetMathLibrary.MakeRotator` 0.0 0.0 (* _newtrack_0 -180.0)) false false))))

(event `self.Sphere.OnComponentEndOverlap`
  (params (OverlappedComponent :type "PrimitiveComponent Object Reference") (OtherActor :type "Actor Object Reference") (OtherComp :type "PrimitiveComponent Object Reference") (OtherBodyIndex :type Integer))
  (cast `/Game/Blueprints/BP_ThirdPersonCharacterCustom` OtherActor)
  (`GameplayStatics.PlaySoundAtLocation` "/Game/Audio/DoorClosing.DoorClosing" (`SceneComponent.K2_GetComponentLocation` (`self.Sphere`)) (struct) 1.0 1.0 0.0 null null null null)
  (goto _label :!via `ReverseFromEnd`))

(fn `UserConstructionScript`
  (`parent.UserConstructionScript`))