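; Finish-line trigger actor that reports lap times for the custom third-person character.
; On BeginPlay it creates a finish-line timer widget and adds it to the viewport.
; When the character overlaps its box, it prints the real-time seconds since the last crossing and resets that timestamp.
; Other overlapping actors only print a debug failure message; the widget is never updated here.
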(event `self.ReceiveBeginPlay`
  (bind _returnvalue (`|CreateWidget` "/Game/Widgets/W_FinishLineTimer.W_FinishLineTimer_C"))
  (bind _output_get (set `self.W Time Widget` _returnvalue))
  (`UserWidget.AddToViewport` _output_get 0))

(event `self.Box.OnComponentBeginOverlap`
  (params (OverlappedComponent :type "PrimitiveComponent Object Reference") (OtherActor :type "Actor Object Reference") (OtherComp :type "PrimitiveComponent Object Reference") (OtherBodyIndex :type Integer) (bFromSweep :type Boolean) (SweepResult :type "HitResult Structure (by ref)"))
  (cast `/Game/Blueprints/BP_ThirdPersonCharacterCustom` OtherActor
    (:`then`
      (`KismetSystemLibrary.PrintString` (`KismetStringLibrary.Concat_StrStr` "That Lap Took " (`KismetTextLibrary.Conv_TextToString` (`KismetTextLibrary.Conv_DoubleToText` (- (`GameplayStatics.GetRealTimeSeconds`) (`self.LastTimeStamp`)) "HalfToEven" false true 1 324 0 2)) " Seconds!"))
      (set `self.LastTimeStamp` (`GameplayStatics.GetRealTimeSeconds`)))
    (:`CastFailed`
      (`KismetSystemLibrary.PrintString` "DID NOT WORK"))))

(fn `UserConstructionScript`)